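; Path-traced Ultra Volumetrics actor that renders a noise-driven volumetric shape, sphere or box, on its HVol component.
; Construction creates a dynamic instance of the PT material, configures optional fog scattering, then pushes noise, shape, color, motion, godray and distortion settings into the material.
; Scattering uses a native or material post-process method, with box bounds scaled by edge falloff.
; UpdateSequencer re-applies all parameters, including a SequencerTime value, to the material.
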(fn ConstructionScript
  (|ConstructionGraph))

(fn UpdateSequencer
  (CallFunction|Parameters))

(fn Parameters
  (Utilities|SetParameters (Variables|Parameters|GetNoise%20Pattern) (Variables|Parameters|GetPattern%20Mixer) (Variables|Parameters|GetShape%20Type) (Variables|Parameters|GetShape%20Edge%20Falloff) (Variables|Parameters|GetOpacity) (Variables|Parameters|GetNoise%20-%20Scale) (Variables|Parameters|GetNoise%20-%20Contrast) (Variables|Parameters|GetNoise%20-%20Multiply) (Variables|Parameters|GetPanning%20Speed) (Variables|Parameters|GetRotation%20Speed) (Variables|Parameters|GetColor) (Variables|Parameters|GetGodrays%20Amount) (Variables|Parameters|GetGodrays%20Scale) (Variables|Parameters|GetDistortion%20Pattern) (Variables|Parameters|GetDistortion%20Scale) (Variables|Parameters|GetDistortion%20Amount) (Variables|Parameters|GetDistortion%20Z%20Amount) (Variables|Sequencer|GetSequencerTime)))

(fn ComponentProperties
  (bind _returnvalue (Actor|GetActorOfClass "/Game/UltraVolumetrics/Core/PaintMode/Blueprint/BP_UltraVolumetricsPainter.BP_UltraVolumetricsPainter_C"))
  (Utilities|IsValid _returnvalue))

(fn CreateMID
  (bind _returnvalue (Rendering|Material|CreateDynamicMaterialInstance "/Game/UltraVolumetrics/Core/Material/Instances/M_UltraVolumetricsPT_Inst.M_UltraVolumetricsPT_Inst" "None" "None" :!class /Script/Engine.KismetMaterialLibrary))
  (bind _output_get (Variables|Materials|SetMaterial _returnvalue))
  (Rendering|Material|SetMaterial (Variables|Default|GetHVol) 0 _output_get))

(fn Scattering
  (bind _scatterpp (Variables|Default|GetScatterPP))
  (bind _scatterparent (Variables|Default|GetScatterParent))
  (bind _scattering_strength (Variables|FogScattering|GetScattering%20Strength))
  (bind _scatterparent_2 (Variables|Default|GetScatterParent))
  (bind _boxextent (Variables|/Script/Engine.BoxComponent|GetBoxExtent _scatterparent))
  (if (Variables|FogScattering|GetEnable%20Fog%20Scattering?)
    ;[0 0 0] Post processing
    (switch Utilities|FlowControl|Switch|SwitchonEnum_ScatteringMethod (Variables|FogScattering|GetFog%20scattering%20method)
      (:NewEnumerator0
        (CallFunction|UltraVolumetricsScattering _scatterpp _scattering_strength false 0.0))
      (:NewEnumerator1
        (CallFunction|UltraVolumetricsScattering _scatterpp _scattering_strength true 0.0)))
    (switch Utilities|FlowControl|Switch|SwitchonEnum_ShapeType (Variables|Parameters|GetShape%20Type)
      (:NewEnumerator0
        (Components|Box|SetBoxExtent _scatterparent_2 (* (Variables|/Script/Engine.BoxComponent|GetBoxExtent _scatterparent_2) (Math|Float|MapRangeClamped (Variables|Parameters|GetShape%20Edge%20Falloff) 0.0 5.0 1.0 0.55)) true))
      (:NewEnumerator1
        (Components|Box|SetBoxExtent _scatterparent (Math|Vector|MakeVector (.x _boxextent) (.y _boxextent) (* (.z _boxextent) (Math|Float|MapRangeClamped (Variables|Parameters|GetShape%20Edge%20Falloff) 0.0 5.0 1.0 0.75))) true)))
    (else
      (Variables|/Script/Engine.PostProcessComponent|SetbEnabled (Variables|Default|GetScatterPP) false)
      (Components|Box|SetBoxExtent (Variables|Default|GetScatterParent) "0, 0, 0" true))))