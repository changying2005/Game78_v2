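; Level manager that runs chapter progression, from the Yellow Turban Rebellion to the Battle of Red Cliffs.
; BeginPlay caches player and first-level enemy spawn points, then teleports the player behind a screen-fade title with movement locked.
; BeginLevel spawns enemies and tracks their deaths; clearing them notifies the BP_Cat task NPC and increments the level index.
; DoTP repeats the titled teleport for chapter two; neither it nor BeginLevel is called here.
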(event Custom|DoTP
  (bind _returnvalue (Game|GetPlayerController 0))
  ;[0.1684 0.1684 0.1684 1 68] 第二关
  (Default|PlayScreenMessage (stale EventBeginPlay _returnvalue_2) "第二章 赤壁之战")
  (Input|SetIgnoreMoveInput _returnvalue true)
  (Utilities|FlowControl|Delay 1.5)
  (Transformation|SetActorLocationAndRotation (Game|GetPlayerCharacter 0) (Utilities|Array|Get(acopy) (Variables|Default|GetPlayerSpawnPosition) (Variables|Default|GetCurrentLevelIndex)))
  (Utilities|FlowControl|Delay 3.0)
  (Input|SetIgnoreMoveInput _returnvalue false))

(event Custom|BeginLevel
  (bind _spawnposition (Variables|Default|GetSpawnPosition))
  ;[0.1684 0.1684 0.1684 1 68] 第一关
  (for _index (range 0 (- (Utilities|Array|Length _spawnposition) 1))
    (bind _returnvalue (Game|SpawnActorfromClass (Variables|Default|GetEnemyClass) (Math|Conversions|ToTransform(Vector) (Utilities|Array|Get(acopy) _spawnposition _index)) "Undefined" "MultiplyWithRoot" 0 0))
    (bind _asenemy_character (Utilities|Casting|CastToEnemyCharacter _returnvalue))
    (EventDispatchers|BindEventtoOnDeathInstant _asenemy_character (delegate Custom|OnDeathInstant_事件))
    (Utilities|Array|Add (Variables|Default|GetActiveEnemies) _returnvalue)))

(event Custom|OnDeathInstant_事件
  (params (dieActor :type Enemy%20Character%20Object%20Reference))
  (bind _activeenemies (Variables|Default|GetActiveEnemies))
  ;[0.1684 0.1684 0.1684 1 68] 第一关
  (Development|PrintString "角色减一")
  (Utilities|Array|RemoveItem _activeenemies dieActor)
  (if (<= (Utilities|Array|Length _activeenemies) 0)
    (Development|PrintString "下一关")
    (bind _asbp_cat (Utilities|Casting|CastToBP_Cat (Variables|Default|GetTaskNPC)))
    (Default|FinishedLevel _asbp_cat (Variables|Default|GetCurrentLevelIndex))
    (bind _result (Math|Integer|IncrementInt (Variables|Default|GetCurrentLevelIndex))
      (:%20%20
        (Variables|Default|SetCurrentLevelIndex _result)))))

(event EventBeginPlay
  (bind _returnvalue (Game|GetPlayerController 0))
  (CallFunction|初始化每关玩家出生点)
  (CallFunction|初始化第一关敌人刷新点位)
  (bind _returnvalue_2 (UserInterface|CreateWidget "/Game/GamePlay/UI/Widgets/ChangeLevel/WB_ScreenFade.WB_ScreenFade_C" _returnvalue))
  (UserInterface|Viewport|AddtoViewport _returnvalue_2 0)
  (Default|PlayScreenMessage _returnvalue_2 "第一章 黄巾起义")
  (Input|SetIgnoreMoveInput _returnvalue true)
  (Utilities|FlowControl|Delay 1.5)
  ;[0.1684 0.1684 0.1684 1 68] 第一关
  (Utilities|Array|Clear (Variables|Default|GetActiveEnemies))
  (Transformation|SetActorLocationAndRotation (Game|GetPlayerCharacter 0) (Utilities|Array|Get(acopy) (Variables|Default|GetPlayerSpawnPosition) (Variables|Default|GetCurrentLevelIndex)))
  (Utilities|FlowControl|Delay 3.0)
  (Input|SetIgnoreMoveInput _returnvalue false))

(event Collision|EventActorBeginOverlap
  (params (OtherActor :type Actor%20Object%20Reference)))

(event EventTick
  (params (DeltaSeconds :type Float%20%28single-precision%29)))

(fn ConstructionScript)

(fn 初始化每关玩家出生点
  (bind _playerspawnpoints (Variables|Default|GetPlayerSpawnPoints))
  (for _index (range 0 (- (Utilities|Array|Length _playerspawnpoints) 1))
    (Utilities|Array|Add (Variables|Default|GetPlayerSpawnPosition) (.Location (Math|Transform|BreakTransform (Transformation|GetActorTransform (Utilities|Array|Get(acopy) _playerspawnpoints _index)))))))

(fn 初始化第一关敌人刷新点位
  (bind _level1spawnpoints (Variables|Default|GetLevel1SpawnPoints))
  (for _index (range 0 (- (Utilities|Array|Length _level1spawnpoints) 1))
    (Development|PrintString (Utilities|String|ToString(Integer) _index))
    (Development|PrintString (Utilities|String|ToString(Vector) (.Location (Math|Transform|BreakTransform (Transformation|GetActorTransform (Utilities|Array|Get(acopy) _level1spawnpoints _index))))))
    (Utilities|Array|Add (Variables|Default|GetSpawnPosition) (.Location (Math|Transform|BreakTransform (Transformation|GetActorTransform (Utilities|Array|Get(acopy) _level1spawnpoints _index)))))))