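; BP_CatGirl_Gamemode_v2 is a game mode that tracks and respawns the cat girl player character.
; On BeginPlay it caches the first BP_CatGril_Character_v2 found in the level as Newpawn.
; RespawnPlayer sets the BPState state to Player.State.Alive, spawns a new character at the given transform, stores it as Newpawn and has player controller 0 possess it.
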(event Custom|Respawn%20Player
  (params (SpawnTransform :type Transform))
  (Default|SetState (Variables|Default|GetBP_State) "(TagName=\"Player.State.Alive\")")
  (bind _returnvalue (Game|SpawnActorfromClass "/Game/GamePlay/Characters/Player/BP_CatGril_Character_v2.BP_CatGril_Character_v2_C" SpawnTransform "Undefined" "MultiplyWithRoot" 0 0))
  (bind _output_get (Variables|Default|SetNewpawn _returnvalue))
  (Pawn|Possess (Game|GetPlayerController 0) _output_get))

(event EventBeginPlay
  (Utilities|FlowControl|DoOnce false
    (:Completed
      (bind _outactors (Actor|GetAllActorsOfClass "/Game/GamePlay/Characters/Player/BP_CatGril_Character_v2.BP_CatGril_Character_v2_C"))
      (Variables|Default|SetNewpawn (Utilities|Array|Get(acopy) _outactors)))))

(fn ConstructionScript)