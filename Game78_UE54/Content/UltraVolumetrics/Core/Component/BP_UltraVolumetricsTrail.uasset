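; Ultra Volumetrics component that attaches a Niagara trail to its owner, using a character or object system depending on whether the owner has a valid Instigator.
; It waits for BP_InteractionController to be ready, then spawns the trail and feeds it size, opacity and persistence.
; Optional Tick records fall speed and fires a one-shot landing burst scaled by velocity and trail size.
; A debug sphere can show the trail offset.
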(event Custom|UpdateParameters
  (bind _trailref (Variables|Default|GetTrailRef))
  (Niagara|SetNiagaraVariable(Float) _trailref "TrailSize" (Variables|Default|GetTrailSize))
  (Niagara|SetNiagaraVariable(Float) _trailref "Opacity" (Variables|Default|GetTrailOpacity))
  (Niagara|SetNiagaraVariable(Float) _trailref "Persistence" (Variables|Default|GetTrailPersistence)))

(event EventBeginPlay
  (bind _offset (Variables|Default|GetOffset))
  (|DebugLocation)
  (|ReadyCheck
    (:Ready
      (Components|Tick|SetComponentTickEnabled (Variables|Default|GetEnableOnLandedEffect?))
      (Utilities|IsValid (Variables|/Script/Engine.Actor|GetInstigator (Components|GetOwner))
        (:Is%20Valid
          (Variables|Default|SetIsCharacter? true))
        (:Is%20Not%20Valid
          (Variables|Default|SetIsCharacter? false)))
      (bind _nsref (CallFunction|UltraVolumetricsSystemAttached (select (Variables|Default|GetIsCharacter?) "/Game/UltraVolumetrics/Core/Niagara/NS_TrailCharacter.NS_TrailCharacter" "/Game/UltraVolumetrics/Core/Niagara/NS_TrailObjects.NS_TrailObjects") (Variables|/Script/Engine.Actor|GetRootComponent (Components|GetOwner)) (Math|Vector|MakeVector (.x _offset) (.y _offset) 0.0) "0, 0, 0" false))
      (bind _output_get (Variables|Default|SetTrailRef _nsref))
      (Utilities|IsValid _output_get
        (:Is%20Valid
          (if (Variables|Default|GetIsCharacter?)
            _
            (else
              (Class|NiagaraComponent|SetVariableBool (Variables|Default|GetTrailRef) "IgnoreZ" true)))
          (Niagara|SetNiagaraVariable(Float) (Variables|Default|GetTrailRef) "TrailSize" (Variables|Default|GetTrailSize))
          (Niagara|SetNiagaraVariable(Float) (Variables|Default|GetTrailRef) "Opacity" (Variables|Default|GetTrailOpacity))
          (Niagara|SetNiagaraVariable(Float) (Variables|Default|GetTrailRef) "Persistence" (Variables|Default|GetTrailPersistence)))))))

(event EventTick
  (params (DeltaSeconds :type Float%20%28single-precision%29))
  (bind _returnvalue (Components|GetOwner))
  (bind _returnvalue_2 (Components|GetOwner))
  (bind _offset (Variables|Default|GetOffset))
  (bind _returnvalue_3 (Transformation|GetVelocity _returnvalue))
  (bind _returnvalue_4 (Transformation|GetVelocity _returnvalue_2))
  (if (< (.z _returnvalue_3) 0.0)
    (Variables|Default|SetZVel (Math|Float|Clamp(Float) (.z _returnvalue_3) -2e+03 -1e+01))
    (goto _label Reset)
    (else
      (Utilities|FlowControl|DoOnce false :!label _label
        (:Completed
          (bind _nsref (CallFunction|UltraVolumetricsSystemAttached "/Game/UltraVolumetrics/Core/Niagara/NS_Jump.NS_Jump" (Variables|/Script/Engine.Actor|GetRootComponent (Components|GetOwner)) (Math|Vector|MakeVector (.x _offset) (.y _offset) 0.0) "0, 0, 0" true))
          (Utilities|IsValid _nsref
            (:Is%20Valid
              (Niagara|SetNiagaraVariable(Vector3) _nsref "Velocity" (* (Math|Vector|MakeVector (.x _returnvalue_4) (.y _returnvalue_4) 0.0) (Math|Float|SelectFloat 2.0 4.0 (Variables|Default|GetIsCharacter?))))
              (Niagara|SetNiagaraVariable(Float) _nsref "Force" (/ (Math|Float|Absolute(Float) (Variables|Default|GetZVel)) (Math|Float|SelectFloat 1.5e+02 5e+01 (Variables|Default|GetIsCharacter?))))
              (Niagara|SetNiagaraVariable(Float) _nsref "Size" (/ (Math|Float|Clamp(Float) (Variables|Default|GetTrailSize) 75.0 2.5e+02) 5e+01)))))))))

(event Custom|DebugUpdate
  (bind _offset (Variables|Default|GetOffset))
  (Rendering|Debug|DrawDebugSphere (Math|Transform|TransformLocation (Transformation|GetActorTransform (Components|GetOwner)) (Math|Vector|MakeVector (.x _offset) (.y _offset) 0.0)) (* (Variables|Default|GetTrailSize) 0.75) 12 "(R=1.000000,G=0.550000,B=0.000000,A=1.000000)" 0.0 5.0))