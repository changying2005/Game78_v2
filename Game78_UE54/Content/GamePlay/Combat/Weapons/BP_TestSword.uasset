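; BP_TestSword is a test sword weapon that delivers hits to combat targets through a HitBox overlap.
; When HitBox overlaps an actor implementing BPI_CombatTarget, it builds an SHitInfo from Damage and OwnerCharacter and sends it through OnReceiveHitMessage.
; Getters expose damage, owner, and fixed weapon and attack types, while attack and interaction checks always return false and the attack source is empty.
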(event OnComponentBeginOverlap(HitBox)
  (params (OverlappedComponent :type Primitive%20Component%20Object%20Reference) (OtherActor :type Actor%20Object%20Reference) (OtherComp :type Primitive%20Component%20Object%20Reference) (OtherBodyIndex :type Integer) (bFromSweep :type Boolean) (SweepResult :type Hit%20Result%20Structure%20%28by%20ref%29))
  (if (Utilities|DoesObjectImplementInterface OtherActor "/Game/GamePlay/Core/Interfaces/BPI_CombatTarget.BPI_CombatTarget_C")
    (bind _hit (CallFunction|GetHitInfoforTarget OtherActor))
    (Class|BPICombatTarget|OnReceiveHit(Message) OtherActor _hit)))

(event EventBeginPlay)

(event Collision|EventActorBeginOverlap
  (params (OtherActor :type Actor%20Object%20Reference)))

(event EventTick
  (params (DeltaSeconds :type Float%20%28single-precision%29)))

(fn ConstructionScript)

(fn CanAttack
  (return false))

(fn CanInteract
  (params (Interactor :type Actor%20Object%20Reference))
  (return false))

(fn GetAttackSource
  (return 0))

(fn GetAttackType
  (return "NewEnumerator0"))

(fn GetDamage
  (return (Variables|Default|GetDamage)))

(fn GetHitInfoforTarget
  (params (Target :type Actor%20Object%20Reference))
  (return (Utilities|Struct|MakeS_HitInfo (Variables|Default|GetDamage) (Variables|Default|GetOwnerCharacter) 0)))

(fn GetInteractText
  (return ""))

(fn GetOwnerCharacter
  (return (Variables|Default|GetOwnerCharacter)))

(fn GetWeaponType
  (return "NewEnumerator0"))