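; BP_Pickup is a data-driven pickup that passes its actor class to the player character on overlap.
; On BeginPlay it reads its DataTable row and async loads the display mesh and the actor class to grant.
; A looping timer bobs and spins the mesh using game time.
; Overlap by the player sends the class through AddWeaponClassMessage, prints a debug string, clears the timer and destroys the pickup.
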(event OnComponentBeginOverlap(Sphere)
  (params (OverlappedComponent :type Primitive%20Component%20Object%20Reference) (OtherActor :type Actor%20Object%20Reference) (OtherComp :type Primitive%20Component%20Object%20Reference) (OtherBodyIndex :type Integer) (bFromSweep :type Boolean) (SweepResult :type Hit%20Result%20Structure%20%28by%20ref%29))
  (if (== OtherActor (Game|GetPlayerCharacter 0))
    (Class|BPIWeaponHolder|AddWeaponClass(Message) OtherActor (Variables|Default|GetPickUp))
    (Development|PrintString "已触碰到pickups")
    (Utilities|Time|ClearandInvalidateTimerbyHandle (Variables|Default|GetRotateTimer))
    (Actor|DestroyActor)))

(event Custom|Rotate
  (bind _returnvalue (Utilities|Time|SetTimerbyEvent (delegate Custom|RotateLoop) 0.01 true))
  (Variables|Default|SetRotateTimer _returnvalue))

(event Custom|RotateLoop
  (CallFunction|Spin "1.000000,1.000000,1.000000"))

(event EventBeginPlay
  (bind _pickupinfo (Variables|Default|GetPickupInfo))
  (bind (_datatable _rowname) (Utilities|Struct|BreakDataTableRowHandle _pickupinfo))
  (bind _returnvalue (Utilities|GetDataTableRow _datatable _rowname)
    (:then
      (Utilities|FlowControl|Sequence
        (:then_0
          (bind _object (Utilities|AsyncLoadAsset (.StaticMesh (Utilities|Struct|BreakS_weapondetails _returnvalue)))
            (:Completed
              (bind _as静态网格体 (Utilities|Casting|CastToStaticMesh _object))
              (Components|StaticMesh|SetStaticMesh (Variables|Default|GetStaticMesh) _as静态网格体))))
        (:then_1
          (bind _class (Utilities|AsyncLoadClassAsset (.SpawnActor (Utilities|Struct|BreakS_weapondetails _returnvalue)))
            (:Completed
              (bind _asactor (Utilities|Casting|CastToActorClass _class))
              (Variables|Default|SetPickUp _asactor))))
        (:then_2
          (CallFunction|Rotate))))))

(fn ConstructionScript)

(fn Spin
  (params (Transform%20Scale :type Vector :default "1.000000,1.000000,1.000000"))
  (bind _returnvalue (Utilities|Time|GetGameTimeinSeconds))
  (Transformation|SetRelativeTransform (Variables|Default|GetStaticMesh) (Math|Transform|MakeTransform (Math|Vector|MakeVector 0.0 0.0 (* (Math|Trig|Sin(Radians) (* _returnvalue 3.0)) 15.0)) (Math|Rotator|MakeRotator 0.0 0.0 (* _returnvalue 1e+02)) Transform%20Scale) false false))