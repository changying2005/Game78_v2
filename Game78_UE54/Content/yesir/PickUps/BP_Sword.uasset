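; Sword weapon Blueprint that plays a three-stage melee combo when AttackBigBegin fires and the weapon is not sheathed.
; AttackIndex selects each section of the PrimaryA attack montage and resets when a montage completes or the third stage starts.
; Montage notifies drive the combo and attacking flags and, in the first two stages only, toggle HitBox collision.
; The IsAttacking and CanSaveCombo checks are disconnected, so neither flag gates attacks here.
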(event Custom|AttackBigBegin
  (params (CurrentWeapon :type Actor%20Object%20Reference))
  (bind _mesh_to_play_on (Variables|Default|GetMesh%20to%20Play%20On))
  ;[0.2031 0.2031 0.2031] 连招三段逻辑
  (if (not (Variables|Default|GetSheathed))
    (if (== (Variables|Default|GetAttackIndex) 0)
      (bind _notifyname (Animation|Montage|PlayMontage _mesh_to_play_on "/Game/GamePlay/animations/Attack/LightAttack/A_Attack_PrimaryA_Montage.A_Attack_PrimaryA_Montage" 1.0 0.0 "Default")
        (:then
          (Variables|Default|SetCanSaveCombo false)
          (Variables|Default|SetAttackIndex 1))
        (:OnCompleted
          (Variables|Default|SetIsAttacking false :!label _label)
          (Variables|Default|SetCanSaveCombo false)
          (Variables|Default|SetAttackIndex 0))
        (:OnNotifyBegin
          (switch name _notifyname
            (:Attack1Begin
              (Variables|Default|SetCanSaveCombo true)
              (Variables|Default|SetIsAttacking true))
            (:Attack1End
              (Variables|Default|SetCanSaveCombo false)
              (Variables|Default|SetIsAttacking false))
            (:AttackCollisionOn
              (Collision|SetCollisionEnabled (Variables|Default|GetHitBox) "QueryAndProbe" :!label _label_2))
            (:AttackCollisionOff
              (Collision|SetCollisionEnabled (Variables|Default|GetHitBox) "NoCollision" :!label _label_3)))))
      (elif (== (Variables|Default|GetAttackIndex) 1)
        (Variables|Default|SetIsAttacking true)
        (bind _notifyname_2 (Animation|Montage|PlayMontage _mesh_to_play_on "/Game/GamePlay/animations/Attack/LightAttack/A_Attack_PrimaryA_Montage.A_Attack_PrimaryA_Montage" 1.0 0.0 "Attack2")
          (:then
            (Variables|Default|SetCanSaveCombo false)
            (Variables|Default|SetAttackIndex 2))
          (:OnCompleted
            (goto _label))
          (:OnNotifyBegin
            (switch name _notifyname_2
              (:Default
                (Variables|Default|SetCanSaveCombo false)
                (Variables|Default|SetIsAttacking false))
              (:Attack2Begin
                (Variables|Default|SetCanSaveCombo true)
                (Variables|Default|SetIsAttacking true))
              (:AttackCollisionOn
                (goto _label_2))
              (:AttackCollisionOff
                (goto _label_3)))))
        (elif (== (Variables|Default|GetAttackIndex) 2)
          (bind _notifyname_3 (Animation|Montage|PlayMontage _mesh_to_play_on "/Game/GamePlay/animations/Attack/LightAttack/A_Attack_PrimaryA_Montage.A_Attack_PrimaryA_Montage" 1.0 0.0 "Attack3")
            (:then
              (Variables|Default|SetAttackIndex 0))
            (:OnCompleted
              (goto _label))
            (:OnNotifyBegin
              (switch name _notifyname_3
                (:Default
                  (Variables|Default|SetCanSaveCombo false))
                (:Attack2Begin
                  (Variables|Default|SetCanSaveCombo true))))))))))

(event EventBeginPlay
  (|CallParentFunction) ; 此节点被禁用，将不会被调用。\n从引脚连出引线来编译功能。
)

(event Collision|EventActorBeginOverlap
  (params (OtherActor :type Actor%20Object%20Reference))
  (|CallParentFunction OtherActor) ; 此节点被禁用，将不会被调用。\n从引脚连出引线来编译功能。
)

(event EventTick
  (params (DeltaSeconds :type Float%20%28single-precision%29))
  (|CallParentFunction DeltaSeconds) ; 此节点被禁用，将不会被调用。\n从引脚连出引线来编译功能。
)

(fn ConstructionScript
  (|CallParentFunction))