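; BP_Cat is a cat NPC that gates level flow through dialogue.
; Each Talk call advances a line in WB_dialogue, blocking move input until the array ends.
; FinishedLevel switches it from the intro lines to the finish lines.
; After a two-second delay, intro completion calls BeginLevel on BP_LevelManager, while finish completion, which also sets CanTP, calls DoTP.
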(event Custom|FinishedLevel
  (params (LevelNumber :type Integer))
  (Variables|Default|SetIsFinishTask true))

(event EventBeginPlay)

(event Collision|EventActorBeginOverlap
  (params (OtherActor :type Actor%20Object%20Reference)))

(event EventTick
  (params (DeltaSeconds :type Float%20%28single-precision%29)))

(event EventTalk
  (bind _returnvalue (Game|GetPlayerController 0))
  (bind _returnvalue_2 (Game|GetPlayerController 0))
  (if (Variables|Default|GetIsFinishTask)
    (Math|Integer|IncrementInt (Variables|Default|GetTalkIndex_Finish)
      (:%20%20
        (if (< (Variables|Default|GetTalkIndex_Finish) (Utilities|Array|Length (Variables|Default|GetDialogue_Finish)))
          (Variables|Default|GetUI
            (:then
              _)
            (:else
              (bind _returnvalue_3 (UserInterface|CreateWidget "/Game/GamePlay/UI/Widgets/ChatBox/WB_dialogue.WB_dialogue_C" _returnvalue_2))
              (Input|SetIgnoreMoveInput _returnvalue_2 true)
              (bind _output_get (Variables|Default|SetUI _returnvalue_3))
              (UserInterface|Viewport|AddtoViewport _output_get 0)))
          (Rendering|Components|TextRender|SetText (Variables|/Game/GamePlay/UI/Widgets/ChatBox/WB_dialogue.WB_dialogue_C|Get对话文本 (Variables|Default|GetUI)) (Utilities|Text|ToText(String) (Utilities|Array|Get(acopy) (Variables|Default|GetDialogue_Finish) (Variables|Default|GetTalkIndex_Finish))))
          (else
            (Widget|RemovefromParent (Variables|Default|GetUI))
            (Variables|Default|SetTalkIndex_Finish -1)
            (Variables|Default|SetUI 0)
            (Input|SetIgnoreMoveInput _returnvalue_2 false)
            (Variables|Default|SetCanTP true)
            (bind _asbp_level_manager (Utilities|Casting|CastToBP_LevelManager (Variables|Default|GetLevelManager)))
            (Utilities|FlowControl|Delay 2.0)
            (Default|DoTP _asbp_level_manager)))))
    (else
      (Math|Integer|IncrementInt (Variables|Default|GetTalkIndex)
        (:%20%20
          (if (< (Variables|Default|GetTalkIndex) (Utilities|Array|Length (Variables|Default|GetDialogue)))
            (Variables|Default|GetUI
              (:then
                _)
              (:else
                (bind _returnvalue_4 (UserInterface|CreateWidget "/Game/GamePlay/UI/Widgets/ChatBox/WB_dialogue.WB_dialogue_C" _returnvalue))
                (Input|SetIgnoreMoveInput _returnvalue true)
                (bind _output_get_2 (Variables|Default|SetUI _returnvalue_4))
                (UserInterface|Viewport|AddtoViewport _output_get_2 0)))
            (Rendering|Components|TextRender|SetText (Variables|/Game/GamePlay/UI/Widgets/ChatBox/WB_dialogue.WB_dialogue_C|Get对话文本 (Variables|Default|GetUI)) (Utilities|Text|ToText(String) (Utilities|Array|Get(acopy) (Variables|Default|GetDialogue) (Variables|Default|GetTalkIndex))))
            (else
              (Widget|RemovefromParent (Variables|Default|GetUI))
              (Variables|Default|SetTalkIndex -1)
              (Variables|Default|SetUI 0)
              (Input|SetIgnoreMoveInput _returnvalue false)
              (Utilities|FlowControl|Delay 2.0)
              (bind _asbp_level_manager_2 (Utilities|Casting|CastToBP_LevelManager (Variables|Default|GetLevelManager)))
              (Default|BeginLevel _asbp_level_manager_2))))))))

(fn ConstructionScript)

(fn CanInteract
  (params (Interactor :type Actor%20Object%20Reference))
  (return false))

(fn GetInteractText
  (return ""))