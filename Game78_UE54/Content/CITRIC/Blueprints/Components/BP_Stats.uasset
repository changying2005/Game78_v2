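; Stats component that tracks its owner's health and stamina and broadcasts stat updates when they change.
; Taking damage clamps health and, at zero, fires a death dispatcher and sets the owner's BP_State component to the death state.
; Stamina regenerates on a looping timer that a gate-and-delay macro starts or cancels, stopping once the maximum is reached.
; Heal, ApplyDamage, IsAlive and the getters are empty stubs.
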(event Custom|RefreshStamina
  (params (StarStaminaRegenerate :type Boolean))
  (if StarStaminaRegenerate
    (Utilities|Time|SetTimerbyFunctionName 0 "Regenerate Stamina" 0.1 true)
    (else
      (Utilities|Time|ClearTimerbyFunctionName 0 "Regenerate Stamina"))))

(event Custom|Handle%20Stamina%20Regenerate%20Event
  (params (Start%20Refresh%20Stamina :type Boolean) (Duration :type Float%20%28double-precision%29))
  (Utilities|HandleStaminaRegenerate Start%20Refresh%20Stamina Duration))

(event EventBeginPlay)

(event EventTick
  (params (DeltaSeconds :type Float%20%28single-precision%29)))

(fn CheckPlayerHasEnoughStamina
  (params (Staminacost :type Float%20%28double-precision%29))
  (return (>= (Variables|Stamina|GetBaseStamina) Staminacost)))

(fn DecreaseStamina
  (params (Staminacost :type Float%20%28double-precision%29))
  (Variables|Stamina|SetBaseStamina (- (Variables|Stamina|GetBaseStamina) Staminacost))
  (Default|CallUpdatestat "NewEnumerator1"))

(fn RegenerateStamina
  (bind _output_get (Variables|Stamina|SetBaseStamina (+ (Variables|Stamina|GetBaseStamina) (Variables|Stamina|GetStaminaRegenerate))))
  (Default|CallUpdatestat "NewEnumerator1")
  (if (>= _output_get (Variables|Stamina|GetMaxStamina))
    (CallFunction|RefreshStamina false)))

(fn TakeDamage
  (params (Damage%20Amount :type Float%20%28double-precision%29))
  (bind _output_get (Variables|Health|SetBaseHealth (Math|Float|Clamp(Float) (- (Variables|Health|GetBaseHealth) Damage%20Amount) 0.0 (Variables|Health|GetMaxHealth))))
  (Default|CallUpdatestat "NewEnumerator0")
  (if (<= _output_get 0.0)
    (Default|CallDeath)
    (Default|SetState (Actor|GetComponentbyClass (Components|GetOwner) "/Game/CITRIC/Blueprints/Components/BP_State.BP_State_C") "(TagName=\"Player.State.Death\")")))

(fn ApplyDamage
  (params (Hit :type S%20Hit%20Info%20Structure))
  (return 0.0))

(fn GetHealthPercent
  (return 0.0))

(fn GetStamina
  (params (staminain :type Float%20%28double-precision%29))
  (return 0.0))

(fn Heal
  (params (Amount :type Float%20%28double-precision%29))
  (return 0.0))

(fn IsAlive
  (return false))