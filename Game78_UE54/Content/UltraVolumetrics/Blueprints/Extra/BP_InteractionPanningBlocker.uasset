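; BP_InteractionPanningBlocker is a placeable UltraVolumetrics actor that spawns the NS_Blocker effect at its location on BeginPlay.
; It first polls every half second until a BP_InteractionController with a valid SC exists.
; It then passes lifetime, size, turbulence and opacity to the spawned system.
; The construction script adds a size-scaled debug mesh, hidden in game and destroyed after that wait unless Debug is enabled.
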(event EventBeginPlay
  (Components|DestroyComponent (Variables|Default|GetThumb))
  (|ReadyCheck
    (:Ready
      (Utilities|FlowControl|Sequence
        (:then_0
          (bind _nsref (CallFunction|UltraVolumetricsSystem "/Game/UltraVolumetrics/Core/Niagara/NS_Blocker.NS_Blocker" (Transformation|GetActorLocation) "0, 0, 0"))
          (Utilities|IsValid _nsref
            (:Is%20Valid
              (Niagara|SetNiagaraVariable(Float) _nsref "Life" (Variables|Default|GetLifetime))
              (Niagara|SetNiagaraVariable(Float) _nsref "Size" (Variables|Default|GetSize))
              (Niagara|SetNiagaraVariable(Float) _nsref "Turbulence" (Variables|Default|GetTurbulence))
              (Niagara|SetNiagaraVariable(Float) _nsref "Opacity" (Variables|Default|GetOpacity)))))
        (:then_1
          (if (not (Variables|Default|GetDebug?))
            (bind _debugshape (Variables|Default|GetDebugShape)
              (:then
                (Components|DestroyComponent _debugshape))
              (:else))))))))

(fn ConstructionScript
  (|Debug))