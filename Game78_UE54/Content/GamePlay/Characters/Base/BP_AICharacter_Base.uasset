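; BP_AICharacter_Base is a base Blueprint for AI characters, mostly a skeleton with only basic damage and death logic implemented.
; TakeDamage subtracts from Health and calls Die at zero or below, which only disables character movement.
; Sprint, weapon and blackboard-update functions are empty stubs.
; The combat, healing and state-query functions return false or zero, so IsAlive and ApplyDamage are not tied to Health.
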(event EventBeginPlay)

(event Collision|EventActorBeginOverlap
  (params (OtherActor :type Actor%20Object%20Reference)))

(event EventTick
  (params (DeltaSeconds :type Float%20%28single-precision%29)))

(fn ConstructionScript)

(fn TakeDamage
  (params (DamageAmount :type Float%20%28double-precision%29))
  (bind _output_get (Variables|Default|SetHealth (- (Variables|Default|GetHealth) DamageAmount)))
  (if (<= _output_get 0.0)
    (CallFunction|Die)))

(fn Die
  (Pawn|Components|CharacterMovement|DisableMovement (Variables|Character|GetCharacterMovement)))

(fn Sprint)

(fn StopSprint)

(fn FireWeapon)

(fn ReloadWeapon)

(fn UpdateBlackboardKeys)

(fn ApplyDamage
  (params (Hit :type S%20Hit%20Info%20Structure))
  (return 0.0))

(fn CanbeAttacked
  (params (Attacker :type Actor%20Object%20Reference))
  (return false))

(fn CanMove
  (return false))

(fn CanRoll
  (return false))

(fn GetMoveSpeed
  (return 0.0))

(fn Heal
  (params (Amount :type Float%20%28double-precision%29))
  (return 0.0))

(fn IsAlive
  (return false))

(fn OnReceiveHit
  (params (Hit :type S%20Hit%20Info%20Structure))
  (return 0.0))