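; AC_Kick is a component that gives the cat-girl player character a flying kick, commented as triggered by the 1 key.
; BeginPlay caches the player pawn as a Character.
; The Kick event plays the front kick montage on its mesh anim instance, setting IsKicking and clearing IsCanMove until a delay equal to the montage's returned length ends, which blocks re-entry during the kick.
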(event Custom|Kick
  ;[1 1 1] 按1实现飞踢
  (if (not (Variables|Default|GetIsKicking))
    (Variables|Default|SetIsKicking true)
    (Variables|Default|SetIsCanMove false)
    (bind _returnvalue (Animation|Montage|MontagePlay (Components|SkeletalMesh|GetAnimInstance (Variables|/Script/Engine.Character|GetMesh (stale EventBeginPlay _output_get))) "/Game/changying/Catgirl_Anims/Anims/Kick/CatGirl_Anim_CO_KI1_front1_Montage.CatGirl_Anim_CO_KI1_front1_Montage" 1.0 "MontageLength" 0.0 true))
    (Utilities|FlowControl|Delay _returnvalue)
    (Variables|Default|SetIsKicking false)
    (Variables|Default|SetIsCanMove true)))

(event EventBeginPlay
  (bind _as角色 (Utilities|Casting|CastToCharacter (Game|Player|GetPlayerPawn 0)))
  (bind _output_get (Variables|Default|SetAs角色 _as角色)))

(event EventTick
  (params (DeltaSeconds :type Float%20%28single-precision%29)))