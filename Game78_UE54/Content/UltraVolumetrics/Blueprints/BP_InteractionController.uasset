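; Interaction controller actor for UltraVolumetrics that feeds gameplay interactions into the effect's material parameter collection.
; An optional top-down scene capture follows the player or actor, snapped to texel steps to avoid swimming, and publishes its position for 2D trails.
; Events write flashlight, line, grenade, ten timeline-faded projectile slots and a ring drawn to a render target.
; Performance saver mode toggles capture, tick and the Niagara capture flag through ToggleTick.
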(event EventLine3dLocations
  (params (StartPoint :type Vector :default "0, 0, 0") (EndPoint :type Vector :default "0, 0, 0"))
  ;[1 0.2368 0 1 75] Extended features
  ;;[0 0 0] Line3d
  (Rendering|Material|SetVectorParameterValue "/Game/UltraVolumetrics/Core/Material/MPC_UltraVolumetrics.MPC_UltraVolumetrics" "LineStart" (Math|Conversions|ToLinearColor(Vector) StartPoint) :!class /Script/Engine.KismetMaterialLibrary)
  (Rendering|Material|SetVectorParameterValue "/Game/UltraVolumetrics/Core/Material/MPC_UltraVolumetrics.MPC_UltraVolumetrics" "LineEnd" (Math|Conversions|ToLinearColor(Vector) EndPoint) :!class /Script/Engine.KismetMaterialLibrary))

(event EventLine3dWidth
  (params (Width :type Float%20%28double-precision%29))
  ;[1 0.2368 0 1 75] Extended features
  ;;[0 0 0] Line3d
  (Rendering|Material|SetScalarParameterValue "/Game/UltraVolumetrics/Core/Material/MPC_UltraVolumetrics.MPC_UltraVolumetrics" "LineWidth" Width :!class /Script/Engine.KismetMaterialLibrary))

(event EventGrenade
  (params (Location :type Vector :default "0, 0, 0") (Radius :type Float%20%28double-precision%29))
  ;[1 0.2368 0 1 75] Extended features
  ;;[0 0 0] 3d Grenade / sphere
  (Rendering|Material|SetVectorParameterValue "/Game/UltraVolumetrics/Core/Material/MPC_UltraVolumetrics.MPC_UltraVolumetrics" "GrenadeLocationRadius" (Utilities|Struct|MakeLinearColor (.x Location) (.y Location) (.z Location) Radius) :!class /Script/Engine.KismetMaterialLibrary))

(event EventFlashlight-Strength
  (params (Strength :type Float%20%28double-precision%29))
  ;[1 0.2368 0 1 75] Extended features
  ;;[0 0 0] Flashight
  (Rendering|Material|SetScalarParameterValue "/Game/UltraVolumetrics/Core/Material/MPC_UltraVolumetrics.MPC_UltraVolumetrics" "FL-Strength" Strength :!class /Script/Engine.KismetMaterialLibrary))

(event EventFlashlight
  (params (StartLocation :type Vector :default "0, 0, 0") (EndLocation :type Vector :default "0, 0, 0") (ConeAngle :type Float%20%28double-precision%29))
  ;[1 0.2368 0 1 75] Extended features
  ;;[0 0 0] Flashight
  (Rendering|Material|SetVectorParameterValue "/Game/UltraVolumetrics/Core/Material/MPC_UltraVolumetrics.MPC_UltraVolumetrics" "FL-Start" (Math|Conversions|ToLinearColor(Vector) StartLocation) :!class /Script/Engine.KismetMaterialLibrary)
  (Rendering|Material|SetVectorParameterValue "/Game/UltraVolumetrics/Core/Material/MPC_UltraVolumetrics.MPC_UltraVolumetrics" "Fl-End" (Math|Conversions|ToLinearColor(Vector) EndLocation) :!class /Script/Engine.KismetMaterialLibrary)
  (Rendering|Material|SetScalarParameterValue "/Game/UltraVolumetrics/Core/Material/MPC_UltraVolumetrics.MPC_UltraVolumetrics" "FL-ConeAngle" ConeAngle :!class /Script/Engine.KismetMaterialLibrary))

(event EventDrawRing
  (params (Texture :type Texture%202D%20Object%20Reference) (TextureChannel :type Linear%20Color%20Structure) (Location :type Vector :default "0, 0, 0") (RotationSpeed :type Float%20%28double-precision%29) (Radius :type Float%20%28double-precision%29) (Lifetime :type Float%20%28double-precision%29))
  ;[1 0.2368 0 1 75] Extended features
  ;;[0 0 0] Vortex 3d
  (|RingGraph Texture TextureChannel Location RotationSpeed Radius Lifetime))

(event EventBeginPlay
  ;[0.2969 0 0] Beginplay
  (CallFunction|InitializeCapture))

(fn ConstructionScript
  (|ConstructionGraph))

(fn InitializeCapture
  (Rendering|ClearRenderTarget2D "/Game/UltraVolumetrics/Core/Textures/T_RT.T_RT")
  (Components|DestroyComponent (Variables|Default|GetThumb))
  (Rendering|Material|SetVectorParameterValue "/Game/UltraVolumetrics/Core/Material/MPC_UltraVolumetrics.MPC_UltraVolumetrics" "RTDistortionAmount" (Utilities|Struct|MakeLinearColor (Variables|Default|GetRT-Distortion-UVscale) (Variables|Default|GetRT-Distortion-Amount) (Variables|Default|GetRT-Distortion-Contrast) 0.015) :!class /Script/Engine.KismetMaterialLibrary)
  (Rendering|Material|SetVectorParameterValue "/Game/UltraVolumetrics/Core/Material/MPC_UltraVolumetrics.MPC_UltraVolumetrics" "TrailVis" (Utilities|Struct|MakeLinearColor 0.3 0.2 (Variables|Default|GetRT-HeightCutoff) (Math|Conversions|ToFloat(Boolean) (Variables|Default|GetInvertTrails))) :!class /Script/Engine.KismetMaterialLibrary)
  (if (Variables|Default|GetEnable2dInteractions?)
    (bind _returnvalue (AddComponent|AddSceneCaptureComponent2D false (Math|Transform|MakeTransform "0, 0, 0" "-90.000000,90.000000, 0" "1.000000,1.000000,1.000000")))
    (Variables|Default|SetSC _returnvalue)
    (if (Variables|Default|GetPerformanceSaverMode?)
      (Actor|Tick|SetActorTickEnabled false)
      (else
        (Actor|Tick|SetActorTickEnabled true)))
    (else
      (Variables|/Script/Engine.SceneCaptureComponent|SetbCaptureOnMovement (Variables|Default|GetSC) false)
      (Variables|/Script/Engine.SceneCaptureComponent|SetbCaptureEveryFrame (Variables|Default|GetSC) false))))

(fn SetProjectileParams
  (params (Start :type Vector) (End :type Vector) (Size :type Float%20%28double-precision%29) (ProjectileName :type String))
  (bind (_x _y _z) (Math|Vector|BreakVector Start))
  (Rendering|Material|SetVectorParameterValue "/Game/UltraVolumetrics/Core/Material/MPC_UltraVolumetrics.MPC_UltraVolumetrics" (Utilities|String|StringToName (Utilities|String|Append ProjectileName "-Start")) (Math|Color|MakeColor _x _y _z Size) :!class /Script/Engine.KismetMaterialLibrary)
  (Rendering|Material|SetVectorParameterValue "/Game/UltraVolumetrics/Core/Material/MPC_UltraVolumetrics.MPC_UltraVolumetrics" (Utilities|String|StringToName (Utilities|String|Append ProjectileName "-End")) (Math|Conversions|ToLinearColor(Vector) End) :!class /Script/Engine.KismetMaterialLibrary))

(fn SetSCLocation
  (params (Location :type Vector))
  (bind _returnvalue (/ 1.0 512.0))
  (bind _sc (Variables|Default|GetSC))
  (bind _sc_2 (Variables|Default|GetSC))
  (bind _returnvalue_2 (Transformation|GetWorldLocation _sc))
  (bind _orthowidth (Variables|/Script/Engine.SceneCaptureComponent2D|GetOrthoWidth _sc_2))
  (bind _returnvalue_3 (* _orthowidth _returnvalue))
  (bind _returnvalue_4 (/ (.y Location) _returnvalue_3))
  (bind _returnvalue_5 (/ (.x Location) _returnvalue_3))
  (bind _returnvalue_6 (Math|Float|Floor _returnvalue_4))
  (bind _returnvalue_7 (Math|Float|Floor _returnvalue_5))
  (bind _returnvalue_8 (Math|Conversions|ToFloat(Integer) _returnvalue_7))
  (bind _returnvalue_9 (Math|Conversions|ToFloat(Integer) _returnvalue_6))
  (bind _returnvalue_10 (Math|Vector|MakeVector _returnvalue_8 _returnvalue_9 0.0))
  (bind _returnvalue_11 (+ _returnvalue_10 0.5))
  (bind _returnvalue_12 (* _returnvalue_11 _returnvalue_3))
  (bind _returnvalue_13 (- _returnvalue_12 _returnvalue_2))
  (return (Math|Vector|MakeVector (.x _returnvalue_13) (.y _returnvalue_13) 0.0)))

(event EventTick
  (params (DeltaSeconds :type Float%20%28single-precision%29))
  (if (Variables|Default|GetCaptureFollowsPlayer?)
    (Variables|Default|SetLocation (Transformation|GetActorLocation (Game|Player|GetPlayerPawn 0)))
    (else
      (Variables|Default|SetLocation (Transformation|GetActorLocation))))
  (Transformation|SetWorldLocation (Variables|Default|GetSC) (Math|Vector|MakeVector (.x (Variables|Default|GetLocation)) (.y (Variables|Default|GetLocation)) (+ (.z (Variables|Default|GetLocation)) 1024.0)) false false)
  (Transformation|AddWorldOffset (Variables|Default|GetSC) (CallFunction|SetSCLocation (Variables|Default|GetLocation)) false false)
  (Rendering|Material|SetVectorParameterValue "/Game/UltraVolumetrics/Core/Material/MPC_UltraVolumetrics.MPC_UltraVolumetrics" "RTPosition" (Utilities|Struct|MakeLinearColor (.x (Variables|Default|GetLocation)) (.y (Variables|Default|GetLocation)) (.z (Variables|Default|GetLocation)) 1.0) :!class /Script/Engine.KismetMaterialLibrary)
  (if (Variables|Default|GetDebugInteractionZone?)
    (Transformation|SetWorldLocation (Variables|Default|GetDebugBox) (- (Transformation|GetWorldLocation (Variables|Default|GetSC)) "0, 0,1150.000000") false false)))

(event EventToggleTick
  (params (Enabled? :type Boolean))
  (if (Variables|Default|GetPerformanceSaverMode?)
    (if Enabled?
      (Utilities|FlowControl|Sequence
        (:then_0
          (Utilities|Toggle2d true :!label _label))
        (:then_1
          (goto _label Niagara))
        (:then_2
          (Timeline|Interaction2dTimeline Stop
            (:sc
              (Utilities|Toggle2d false :!label _label_2))
            (:particle
              (goto _label_2 Niagara)))))
      (else
        (Timeline|Interaction2dTimeline PlayFromStart)))))

(event EventProjectile5
  (params (Start :type Vector :default "0, 0, 0") (End :type Vector :default "0, 0, 0") (FadeSpeed :type Float%20%28double-precision%29) (Size :type Float%20%28double-precision%29))
  (CallFunction|SetProjectileParams Start End Size "Bullet5")
  (Components|Timeline|SetPlayRate (Variables|Default|GetProjectile5Timeline) FadeSpeed)
  (bind _alpha (Timeline|Projectile5Timeline PlayFromStart)
    (:Update
      (Rendering|Material|SetScalarParameterValue "/Game/UltraVolumetrics/Core/Material/MPC_UltraVolumetrics.MPC_UltraVolumetrics" "Bullet5-Time" (Math|Float|Lerp 0.0 1.0 _alpha) :!class /Script/Engine.KismetMaterialLibrary))))

(event EventProjectile6
  (params (Start :type Vector :default "0, 0, 0") (End :type Vector :default "0, 0, 0") (FadeSpeed :type Float%20%28double-precision%29) (Size :type Float%20%28double-precision%29))
  (CallFunction|SetProjectileParams Start End Size "Bullet6")
  (Components|Timeline|SetPlayRate (Variables|Default|GetProjectile6Timeline) FadeSpeed)
  (bind _alpha (Timeline|Projectile6Timeline PlayFromStart)
    (:Update
      (Rendering|Material|SetScalarParameterValue "/Game/UltraVolumetrics/Core/Material/MPC_UltraVolumetrics.MPC_UltraVolumetrics" "Bullet6-Time" (Math|Float|Lerp 0.0 1.0 _alpha) :!class /Script/Engine.KismetMaterialLibrary))))

(event EventProjectile7
  (params (Start :type Vector :default "0, 0, 0") (End :type Vector :default "0, 0, 0") (FadeSpeed :type Float%20%28double-precision%29) (Size :type Float%20%28double-precision%29))
  (CallFunction|SetProjectileParams Start End Size "Bullet7")
  (Components|Timeline|SetPlayRate (Variables|Default|GetProjectile7Timeline) FadeSpeed)
  (bind _alpha (Timeline|Projectile7Timeline PlayFromStart)
    (:Update
      (Rendering|Material|SetScalarParameterValue "/Game/UltraVolumetrics/Core/Material/MPC_UltraVolumetrics.MPC_UltraVolumetrics" "Bullet7-Time" (Math|Float|Lerp 0.0 1.0 _alpha) :!class /Script/Engine.KismetMaterialLibrary))))

(event EventProjectile8
  (params (Start :type Vector :default "0, 0, 0") (End :type Vector :default "0, 0, 0") (FadeSpeed :type Float%20%28double-precision%29) (Size :type Float%20%28double-precision%29))
  (CallFunction|SetProjectileParams Start End Size "Bullet8")
  (Components|Timeline|SetPlayRate (Variables|Default|GetProjectile8Timeline) FadeSpeed)
  (bind _alpha (Timeline|Projectile8Timeline PlayFromStart)
    (:Update
      (Rendering|Material|SetScalarParameterValue "/Game/UltraVolumetrics/Core/Material/MPC_UltraVolumetrics.MPC_UltraVolumetrics" "Bullet8-Time" (Math|Float|Lerp 0.0 1.0 _alpha) :!class /Script/Engine.KismetMaterialLibrary))))

(event EventProjectile10
  (params (Start :type Vector :default "0, 0, 0") (End :type Vector :default "0, 0, 0") (FadeSpeed :type Float%20%28double-precision%29) (Size :type Float%20%28double-precision%29))
  (CallFunction|SetProjectileParams Start End Size "Bullet10")
  (Components|Timeline|SetPlayRate (Variables|Default|GetProjectile10Timeline) FadeSpeed)
  (bind _alpha (Timeline|Projectile10Timeline PlayFromStart)
    (:Update
      (Rendering|Material|SetScalarParameterValue "/Game/UltraVolumetrics/Core/Material/MPC_UltraVolumetrics.MPC_UltraVolumetrics" "Bullet10-Time" (Math|Float|Lerp 0.0 1.0 _alpha) :!class /Script/Engine.KismetMaterialLibrary))))

(event EventProjectile9
  (params (Start :type Vector :default "0, 0, 0") (End :type Vector :default "0, 0, 0") (FadeSpeed :type Float%20%28double-precision%29) (Size :type Float%20%28double-precision%29))
  (CallFunction|SetProjectileParams Start End Size "Bullet9")
  (Components|Timeline|SetPlayRate (Variables|Default|GetProjectile9Timeline) FadeSpeed)
  (bind _alpha (Timeline|Projectile9Timeline PlayFromStart)
    (:Update
      (Rendering|Material|SetScalarParameterValue "/Game/UltraVolumetrics/Core/Material/MPC_UltraVolumetrics.MPC_UltraVolumetrics" "Bullet9-Time" (Math|Float|Lerp 0.0 1.0 _alpha) :!class /Script/Engine.KismetMaterialLibrary))))

(event EventProjectile1
  (params (Start :type Vector :default "0, 0, 0") (End :type Vector :default "0, 0, 0") (FadeSpeed :type Float%20%28double-precision%29) (Size :type Float%20%28double-precision%29))
  (CallFunction|SetProjectileParams Start End Size "Bullet1")
  (Components|Timeline|SetPlayRate (Variables|Default|GetProjectile1Timeline) FadeSpeed)
  (bind _alpha (Timeline|Projectile1Timeline PlayFromStart)
    (:Update
      (Rendering|Material|SetScalarParameterValue "/Game/UltraVolumetrics/Core/Material/MPC_UltraVolumetrics.MPC_UltraVolumetrics" "Bullet1-Time" (Math|Float|Lerp 0.0 1.0 _alpha) :!class /Script/Engine.KismetMaterialLibrary))))

(event EventProjectile2
  (params (Start :type Vector :default "0, 0, 0") (End :type Vector :default "0, 0, 0") (FadeSpeed :type Float%20%28double-precision%29) (Size :type Float%20%28double-precision%29))
  (CallFunction|SetProjectileParams Start End Size "Bullet2")
  (Components|Timeline|SetPlayRate (Variables|Default|GetProjectile2Timeline) FadeSpeed)
  (bind _alpha (Timeline|Projectile2Timeline PlayFromStart)
    (:Update
      (Rendering|Material|SetScalarParameterValue "/Game/UltraVolumetrics/Core/Material/MPC_UltraVolumetrics.MPC_UltraVolumetrics" "Bullet2-Time" (Math|Float|Lerp 0.0 1.0 _alpha) :!class /Script/Engine.KismetMaterialLibrary))))

(event EventProjectile3
  (params (Start :type Vector :default "0, 0, 0") (End :type Vector :default "0, 0, 0") (FadeSpeed :type Float%20%28double-precision%29) (Size :type Float%20%28double-precision%29))
  (CallFunction|SetProjectileParams Start End Size "Bullet3")
  (Components|Timeline|SetPlayRate (Variables|Default|GetProjectile3Timeline) FadeSpeed)
  (bind _alpha (Timeline|Projectile3Timeline PlayFromStart)
    (:Update
      (Rendering|Material|SetScalarParameterValue "/Game/UltraVolumetrics/Core/Material/MPC_UltraVolumetrics.MPC_UltraVolumetrics" "Bullet3-Time" (Math|Float|Lerp 0.0 1.0 _alpha) :!class /Script/Engine.KismetMaterialLibrary))))

(event EventProjectile4
  (params (Start :type Vector :default "0, 0, 0") (End :type Vector :default "0, 0, 0") (FadeSpeed :type Float%20%28double-precision%29) (Size :type Float%20%28double-precision%29))
  (CallFunction|SetProjectileParams Start End Size "Bullet4")
  (Components|Timeline|SetPlayRate (Variables|Default|GetProjectile4Timeline) FadeSpeed)
  (bind _alpha (Timeline|Projectile4Timeline PlayFromStart)
    (:Update
      (Rendering|Material|SetScalarParameterValue "/Game/UltraVolumetrics/Core/Material/MPC_UltraVolumetrics.MPC_UltraVolumetrics" "Bullet4-Time" (Math|Float|Lerp 0.0 1.0 _alpha) :!class /Script/Engine.KismetMaterialLibrary))))