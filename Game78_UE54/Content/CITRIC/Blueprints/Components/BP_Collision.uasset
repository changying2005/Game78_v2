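; BP_Collision is a component that detects weapon hits while collision is switched on.
; Each tick it sphere-traces for objects between the weapon's start and end sockets, recording new actors and broadcasting DamageActor with the hit.
; Turning collision on clears the already-hit list, so each actor registers once per activation.
; The weapon is supplied through SetWeapon, and PerformAttack is a stub returning zero.
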(event Custom|Collision%20Trace
  (bind _weapon (Variables|Default|GetWeapon))
  (bind _outhits (Collision|MultiSphereTraceForObjects (Transformation|GetSocketLocation _weapon (Variables|Default|GetStartsocket)) (Transformation|GetSocketLocation _weapon (Variables|Default|GetEndsocket)) (Variables|Default|GetRadius) (Variables|Default|GetObject%20Types) false (Variables|Default|GetActors%20to%20Ignore) (Variables|Default|GetDraw%20Debug%20Type)))
  (for _array_element _outhits
    (bind _output_get (Variables|Default|SetLasthit _array_element))
    (bind _returnvalue (CallFunction|CanHitActor (.HitActor (Collision|BreakHitResult _output_get))))
    (if _returnvalue
      (bind _output_get_2 (Variables|Default|SetHit%20Actor (.HitActor (Collision|BreakHitResult _output_get))))
      (Utilities|Array|Add (Variables|Default|GetIsAlreadyHit) _output_get_2)
      (Default|CallDamageActor (Variables|Default|GetLasthit)))))

(event Custom|Turn%20On%20Collision
  (CallFunction|ClearHitActor)
  (Variables|Default|SetIsCollisionOn true))

(event Custom|Clear%20Hit%20Actor
  (Utilities|Array|Clear (Variables|Default|GetIsAlreadyHit)))

(event Custom|Turn%20Off%20Collision
  (Variables|Default|SetIsCollisionOn false))

(event Custom|Set%20Weapon
  (params (Weapon :type Primitive%20Component%20Object%20Reference))
  (Variables|Default|SetWeapon Weapon))

(event EventBeginPlay)

(event EventTick
  (params (DeltaSeconds :type Float%20%28single-precision%29))
  (if (Variables|Default|GetIsCollisionOn)
    (CallFunction|CollisionTrace)))

(fn CanHitActor
  (params (Actor :type Actor%20Object%20Reference))
  (return (not (Utilities|Array|ContainsItem (Variables|Default|GetIsAlreadyHit) Actor))))

(fn PerformAttack
  (params (AttackType :type EMontageAct%20Enum :default "NewEnumerator0"))
  (return 0.0))