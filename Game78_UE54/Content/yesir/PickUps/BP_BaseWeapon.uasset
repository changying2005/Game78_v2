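; Base weapon Blueprint for melee weapons that can be equipped, sheathed and swung.
; Equip and unequip attach it to the hand or sheath socket; sheathe toggles do so on montage notifies.
; Unsheathed attacks play the normal montage, whose notifies toggle HitBox collision, with a flag and short delay blocking re-entry.
; HitBox overlaps send damage and owner to BPI_CombatTarget actors; several getters remain stubs.
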(event OnComponentBeginOverlap(HitBox)
  (params (OverlappedComponent :type Primitive%20Component%20Object%20Reference) (OtherActor :type Actor%20Object%20Reference) (OtherComp :type Primitive%20Component%20Object%20Reference) (OtherBodyIndex :type Integer) (bFromSweep :type Boolean) (SweepResult :type Hit%20Result%20Structure%20%28by%20ref%29))
  ;[0.2378 0.2378 0.2378] 武器碰撞判定，发送伤害
  (if (Utilities|DoesObjectImplementInterface OtherActor "/Game/GamePlay/Core/Interfaces/BPI_CombatTarget.BPI_CombatTarget_C")
    (bind _hit (CallFunction|GetHitInfoforTarget OtherActor))
    (Class|BPICombatTarget|OnReceiveHit(Message) OtherActor _hit)))

(event Custom|AttackBegin
  ;[0.158 0.158 0.158] 攻击
  (if (not (Variables|Default|GetSheathed))
    (if (not (Variables|Default|GetIsAttacking))
      (Variables|Default|SetIsAttacking true)
      (bind _notifyname (Animation|Montage|PlayMontage (stale EventEquiporUnequip MeshToPlayOn) (Variables|Default|GetNomralAttack))
        (:OnCompleted
          (Utilities|FlowControl|Delay 0.2)
          (Variables|Default|SetIsAttacking false))
        (:OnNotifyBegin
          (switch name _notifyname
            (:AttackCollisionOn
              (Development|PrintString "开启剑碰撞")
              (Collision|SetCollisionEnabled (Variables|组件|GetHitBox) "QueryAndProbe"))
            (:AttackCollisionOff
              (Development|PrintString "关闭剑碰撞")
              (Collision|SetCollisionEnabled (Variables|组件|GetHitBox) "NoCollision"))))))))

(event EventSetHidden
  (params (SetHidden :type Boolean))
  (Rendering|SetActorHiddenInGame SetHidden))

(event EventSheatheorUnsheathe
  (params (MeshToPlayOn :type Skeletal%20Mesh%20Component%20Object%20Reference))
  ;[0.1128 0.1128 0.1128] 装备武器
  (if (Variables|Default|GetSheathed)
    (Animation|Montage|PlayMontage MeshToPlayOn (Utilities|ResolveSoftReference (Variables|Default|GetEquip))
      (:OnCompleted
        (Variables|Default|SetSheathed false))
      (:OnNotifyBegin
        (Transformation|AttachComponentToComponent self MeshToPlayOn (Variables|Default|GetSword) "SnapToTarget" "SnapToTarget" "SnapToTarget" true)))
    (else
      ;[0.1128 0.1128 0.1128] 卸下武器
      (Variables|Default|SetSheathed true)
      (Animation|Montage|PlayMontage MeshToPlayOn (Utilities|ResolveSoftReference (Variables|Default|GetUnequip))
        (:OnNotifyBegin
          (Transformation|AttachComponentToComponent self MeshToPlayOn (Variables|Default|GetSheathedSocket) "SnapToTarget" "SnapToTarget" "SnapToTarget" true))))))

(event EventEquiporUnequip
  (params (MeshToPlayOn :type Skeletal%20Mesh%20Component%20Object%20Reference) (Unequip :type Boolean))
  ;[0.1997 0.1997 0.1997] 切换武器
  (Variables|Default|SetMesh%20to%20Play%20On MeshToPlayOn)
  (bind _output_get (Variables|Default|SetUnequiped Unequip))
  (Transformation|AttachComponentToComponent self MeshToPlayOn (select _output_get (Variables|Default|GetSheathedSocket) (Variables|Default|GetSword)) "SnapToTarget" "SnapToTarget" "SnapToTarget" true))

(fn ConstructionScript)

(fn GetAttackType
  (return "NewEnumerator0"))

(fn GetDamage
  (return 0.0))

(fn GetHitInfoforTarget
  (params (Target :type Actor%20Object%20Reference))
  (return (Utilities|Struct|MakeS_HitInfo (Variables|Default|GetDamage) (Variables|Default|GetOwnerCharacter) 0)))

(fn GetOwnerCharacter
  (return 0))

(fn IsweaponSheathed
  (return (Variables|Default|GetSheathed)))

(fn WeaponVariables
  (return (Variables|Default|GetNomralAttack) (Variables|Default|GetHeavyAttack) (Variables|Default|GetDamage)))