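; AC_Weapon is a player component that manages owned weapons: equipping, switching, sheathing and attacking.
; EquipWeapon spawns a weapon class not yet owned, stores it, hides the previous one and equips it through message calls.
; InitWeapon caches the current weapon's montages and damage.
; Keys cycle weapons while preserving sheathed state and toggle sheathing; left click calls BP_BaseWeapon's AttackBegin, leaving the component's montage playback unconnected.
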(event Custom|InitWeapon
  (bind (_nomralattack _heavyattack _damage) (Class|BPIWeaponDetails|WeaponVariables(Message) (Variables|Default|GetCurrentWeapon)))
  (Variables|Default|SetCombo%20Attack%20Montage _nomralattack)
  (Variables|Default|SetCharged%20Attack%20Montage _heavyattack)
  (Variables|Default|SetMelee%20Damage _damage))

(event Custom|EquipWeapon
  (params (NewParam :type Actor%20Class%20Reference))
  (bind _returnvalue (Game|Player|GetPlayerPawn 0))
  (bind _output_get (Variables|Default|SetWeapon NewParam))
  (Development|PrintString (Utilities|GetClassDisplayName _output_get))
  (bind _owned (CallFunction|IsweaponOwenedFunction _output_get))
  (if (not _owned)
    (Development|PrintString "开始装备")
    (bind _returnvalue_2 (Game|SpawnActorfromClass _output_get (Transformation|GetActorTransform _returnvalue) "Undefined" "MultiplyWithRoot" _returnvalue _returnvalue))
    (bind _returnvalue_3 (Utilities|Array|Add (Variables|Default|GetOwnedweapons) _returnvalue_2))
    (Variables|Default|SetCurrentWeaponIndex _returnvalue_3)
    (Utilities|FlowControl|Sequence
      (:then_0
        (Utilities|IsValid (Variables|Default|GetCurrentWeapon)
          (:Is%20Valid
            (Class|BPIWeaponDetails|SetHidden(Message) (Variables|Default|GetCurrentWeapon) true))))
      (:then_1
        (bind _output_get_2 (Variables|Default|SetCurrentWeapon _returnvalue_2))
        (Class|BPIWeaponDetails|EquiporUnequip(Message) _output_get_2 (Variables|/Script/Engine.Character|GetMesh (stale EventBeginPlay _output_get)) false)
        (CallFunction|InitWeapon)))))

(event EventBeginPlay
  (bind _as角色 (Utilities|Casting|CastToCharacter (Game|Player|GetPlayerPawn 0)))
  (bind _output_get (Variables|Default|SetPlayer角色 _as角色))
  (Development|PrintString (Utilities|GetClassDisplayName (Utilities|GetClass _output_get))))

(event EventTick
  (params (DeltaSeconds :type Float%20%28single-precision%29)))

(event Input|KeyboardEvents|2
  (params (Key :type Key%20Structure :default "None"))
  ;[1 1 1] 切换武器槽
  (:Pressed
    (bind _currentweapon (Variables|Default|GetCurrentWeapon)
      (:then
        (Class|BPIWeaponDetails|SheatheorUnsheathe(Message) _currentweapon (Variables|/Script/Engine.Character|GetMesh (stale EventBeginPlay _output_get))))
      (:else))))

(event Input|KeyboardEvents|1
  (params (Key :type Key%20Structure :default "None"))
  ;[1 1 1] 切换武器
)

(event Input|MouseEvents|MouseWheelDown
  (params (Key :type Key%20Structure :default "None"))
  ;[1 1 1] 切换武器槽
)

(event Input|MouseEvents|LeftMouseButton
  (params (Key :type Key%20Structure :default "None"))
  (bind _currentweapon (Variables|Default|GetCurrentWeapon))
  ;[1 1 1] 左键调用攻击模块
  (:Pressed
    (Utilities|IsValid _currentweapon
      (:Is%20Valid
        (bind _asbp_base_weapon (Utilities|Casting|CastToBP_BaseWeapon _currentweapon))
        (Default|AttackBegin _asbp_base_weapon)))))

(event Input|KeyboardEvents|E
  (params (Key :type Key%20Structure :default "None"))
  ;[1 1 1] 切换武器
  (:Pressed
    (if (> (Utilities|Array|Length (Variables|Default|GetOwnedweapons)) 1)
      (bind _currentweapon (Variables|Default|GetCurrentWeapon)
        (:then
          (Class|BPIWeaponDetails|SetHidden(Message) _currentweapon true)
          (bind _sheathed (Class|BPIWeaponDetails|IsweaponSheathed(Message) _currentweapon))
          (bind _output_get (Variables|Default|SetCurrentWeaponIndex (Math|Integer|SelectInt 0 (+ (Variables|Default|GetCurrentWeaponIndex) 1) (== (Utilities|Array|LastIndex (Variables|Default|GetOwnedweapons)) (Variables|Default|GetCurrentWeaponIndex)))))
          (bind _output_get_2 (Variables|Default|SetCurrentWeapon (Utilities|Array|Get(acopy) (Variables|Default|GetOwnedweapons) _output_get)))
          (Class|BPIWeaponDetails|EquiporUnequip(Message) _output_get_2 (Variables|/Script/Engine.Character|GetMesh (stale EventBeginPlay _output_get)) _sheathed)
          (Class|BPIWeaponDetails|SetHidden(Message) _output_get_2 false)
          (CallFunction|InitWeapon))
        (:else)))))

(fn IsweaponOwenedFunction
  (params (ObjectClass :type Object%20Class%20Reference))
  (for _array_element (Variables|Default|GetOwnedweapons)
    (if (Class|GameplayStatics|ObjectIsA _array_element ObjectClass)
      (return true _array_element)))
  (return false 0))